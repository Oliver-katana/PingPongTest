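; Game mode that sets up a two-player networked match with a ball as players log in.
; PostLogin stores each controller, then spawns and possesses a pawn at one of the level's PlayerStarts, chosen by join order.
; When the second player joins, short delays lead into SpawnBall and then a game state multicast that removes the waiting widget.
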(event `self.K2_PostLogin`
  (params (NewPlayer :type "PlayerController Object Reference"))
  (bind _playercontrollers (`self.PlayerControllers`))
  (bind _output (`|GetArrayItem` _playercontrollers))
  (bind _output_2 (`|GetArrayItem` (`self.PlayerControllers`) 1))
  ;[1 1 1] Check for both players connected and save their controllers
  (bind _returnvalue (`KismetArrayLibrary.Array_Add` _playercontrollers NewPlayer))
  (if (== _returnvalue 1)
    (bind _returnvalue_2 (`|SpawnActorFromClass` "/Game/MainBPs/MyPawnBP.MyPawnBP_C" (`self.GetTransform` (`|GetArrayItem` (`self.GetPlayerStarts`) 1)) "AlwaysSpawn" "OverrideRootScale" _output_2 null))
    (`Controller.Possess` _output_2 _returnvalue_2)
    (`KismetSystemLibrary.Delay` 0.5)
    (`self.SpawnBall`)
    (`KismetSystemLibrary.Delay` 0.2)
    (bind _asmy_game_state_bp (cast `/Game/MainBPs/MyGameStateBP` (`GameplayStatics.GetGameState`)))
    (`/Game/MainBPs/MyGameStateBP.RemoveWaitingWidget_Multicast` _asmy_game_state_bp (`self.PlayerControllers`))
    (else
      (bind _returnvalue_3 (`|SpawnActorFromClass` "/Game/MainBPs/MyPawnBP.MyPawnBP_C" (`self.GetTransform` (`|GetArrayItem` (`self.GetPlayerStarts`))) "AlwaysSpawn" "OverrideRootScale" _output null))
      (`Controller.Possess` _output _returnvalue_3))))

(fn `GetPlayerStarts`
  (returns (PlayerStarts :type "Array of PlayerStart Object Reference"))
  (bind _outactors (`GameplayStatics.GetAllActorsOfClass` "/Script/Engine.PlayerStart"))
  (return _outactors))

(fn `UserConstructionScript`)