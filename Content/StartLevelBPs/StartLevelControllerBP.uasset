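; Player controller for the start level that shows the menu widget to the local player.
; On BeginPlay it creates the Menu widget, adds it to the viewport, shows the mouse cursor and switches to UI-only input focused on the menu, without locking the mouse.
; When destroyed, it hides the cursor and restores game-only input.
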(event `self.ReceiveBeginPlay`
  (if (`self.IsLocalController`)
    (bind _returnvalue (`|CreateWidget` "/Game/UI/Menu.Menu_C"))
    (bind _output_get (set `self.MenuRef` _returnvalue))
    (`UserWidget.AddToViewport` _output_get 0)
    (set `self.bShowMouseCursor` true)
    (`WidgetBlueprintLibrary.SetInputMode_UIOnlyEx` self _output_get)))

(event `self.ReceiveDestroyed`
  (set `self.bShowMouseCursor` false)
  (`WidgetBlueprintLibrary.SetInputMode_GameOnly` self))

(fn `UserConstructionScript`)